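; BP_panner is an example Blueprint that ties a material parameter on its Sphere component to the player character's position.
; The construction script creates a dynamic material instance from the sphere's first material and stores it as EsferaMat.
; Every tick it sets the VelocidadPan scalar, named as a pan speed, from the player's world X location scaled down by a constant.
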(event `self.ReceiveTick`
  (params (DeltaSeconds :type "Float (single-precision)"))
  (`MaterialInstanceDynamic.SetScalarParameterValue` (`self.EsferaMat`) "VelocidadPan" (/ (.x (`self.K2_GetActorLocation` (`GameplayStatics.GetPlayerCharacter` 0))) 300.0)))

(fn `UserConstructionScript`
  (bind _sphere (`self.Sphere`))
  (bind _returnvalue (`PrimitiveComponent.CreateDynamicMaterialInstance` _sphere 0 (`PrimitiveComponent.GetMaterial` _sphere 0) "None"))
  (set `self.EsferaMat` _returnvalue))